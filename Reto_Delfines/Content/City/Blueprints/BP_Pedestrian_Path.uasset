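; BP_Pedestrian_Path is a city actor that feeds randomly chosen pedestrians (woman, man or pet) onto a spline path.
; While ActivateSpawn is set, BeginPlay and every Tick attempt a spawn just below the spline's first point, once the newest pedestrian has moved at least OffsetBetweenPedestrians along it.
; Each spawn receives the spline and traffic light, then joins the Pedestrians array; the construction script links the array's first entry likewise.
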(event Custom|Begin%20Path
  (if (Variables|Default|GetActivate%20Spawn)
    (CallFunction|SpawnPedestrian)))

(event EventBeginPlay
  (CallFunction|BeginPath))

(event Collision|EventActorBeginOverlap
  (params (OtherActor :type Actor%20Object%20Reference)))

(event EventTick
  (params (DeltaSeconds :type Float%20%28single-precision%29))
  (CallFunction|BeginPath))

(fn ConstructionScript
  (bind _pedestrians (Variables|Default|GetPedestrians))
  (bind _output (Utilities|Array|Get(acopy) _pedestrians))
  (Variables|/Game/City/Blueprints/BP_Pedestrian.BP_Pedestrian_C|SetPath _output (Variables|Default|GetSpline))
  (Variables|/Game/City/Blueprints/BP_Pedestrian.BP_Pedestrian_C|SetTraffic%20%20Light%20to%20Follow _output (Variables|Default|GetTraffic%20Light)))

(fn CheckPedestrianatBegining
  (bind _pedestrians (Variables|Default|GetPedestrians))
  (return (< (Variables|/Game/City/Blueprints/BP_Pedestrian.BP_Pedestrian_C|GetDistance%20Along%20Spline (Utilities|Array|Get(acopy) _pedestrians (Utilities|Array|LastIndex _pedestrians))) (Variables|Default|GetOffset%20between%20Pedestrians))))

(fn AddPedestrian
  (params (Pedestrian :type BP%20Pedestrian%20Object%20Reference))
  (Variables|/Game/City/Blueprints/BP_Pedestrian.BP_Pedestrian_C|SetTraffic%20%20Light%20to%20Follow Pedestrian (Variables|Default|GetTraffic%20Light))
  (Variables|/Game/City/Blueprints/BP_Pedestrian.BP_Pedestrian_C|SetPath Pedestrian (Variables|Default|GetSpline))
  (Utilities|Array|Add (Variables|Default|GetPedestrians) Pedestrian))

(fn GetPedestrianTransform
  (bind _spline (Variables|Default|GetSpline))
  (bind _returnvalue (Spline|GetLocationatSplinePoint _spline 0 "World"))
  (return (Math|Vector|MakeVector (.x _returnvalue) (.y _returnvalue) (+ (.z _returnvalue) -2e+01)) (Spline|GetRotationatSplinePoint _spline 0 "World")))

(fn SpawnPedestrian
  (bind _pedestrian_at_begining_ (CallFunction|CheckPedestrianatBegining))
  (if (not _pedestrian_at_begining_)
    (bind (_location _rotation) (CallFunction|GetPedestrianTransform))
    (switch Utilities|FlowControl|Switch|SwitchonE_Pedestrian (Utilities|Enum|ByteToEnumE_Pedestrian (Math|Conversions|ToByte(Integer) (Math|Random|RandomIntegerinRange 0 2)))
      (:NewEnumerator0
        (bind _returnvalue (Game|SpawnActorfromClass "/Game/City/Blueprints/BP_Woman.BP_Woman_C" (Math|Transform|MakeTransform _location _rotation "1.000000,1.000000,1.000000") "Undefined" "MultiplyWithRoot" 0 0))
        (CallFunction|AddPedestrian _returnvalue))
      (:NewEnumerator1
        (bind _returnvalue_2 (Game|SpawnActorfromClass "/Game/City/Blueprints/BP_Man.BP_Man_C" (Math|Transform|MakeTransform _location _rotation "1.000000,1.000000,1.000000") "Undefined" "MultiplyWithRoot" 0 0))
        (CallFunction|AddPedestrian _returnvalue_2))
      (:NewEnumerator2
        (bind _returnvalue_3 (Game|SpawnActorfromClass "/Game/City/Blueprints/BP_Pet.BP_Pet_C" (Math|Transform|MakeTransform _location _rotation "1.000000,1.000000,1.000000") "Undefined" "MultiplyWithRoot" 0 0))
        (CallFunction|AddPedestrian _returnvalue_3)))))