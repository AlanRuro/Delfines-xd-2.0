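; Traffic light "leader" actor for the city, which competes with a rival light for the green phase based on car demand.
; On BeginPlay it loops: it sums its own and its partner's car counts, then polls until the competitor has updated.
; It goes green then yellow if its preference-weighted count beats the competitor's, otherwise red, using timed delays.
; Each cycle ends by clearing its updated flag and briefly holding red before recounting.
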(event EventBeginPlay
  (CallFunction|GetTotalNumCars :!label _label)
  (bind _is_competitor_updated_ (CallFunction|AskCompetitorforUpdate :!label _label_2))
  (if _is_competitor_updated_
    (bind _won_ (CallFunction|Negotiate))
    (if _won_
      (CallFunction|TurnGreen)
      (Utilities|FlowControl|Delay (Variables|Default|GetDuration))
      (CallFunction|TurnYellow)
      (Utilities|FlowControl|Delay (Variables|Default|GetDuration))
      (else
        (CallFunction|TurnRed)
        (Utilities|FlowControl|Delay (Variables|Default|GetDuration))))
    (Variables|Default|SetUpdated false)
    (CallFunction|TurnRed)
    (Utilities|FlowControl|Delay 0.5)
    (goto _label)
    (else
      (Utilities|FlowControl|Delay 0.2)
      (goto _label_2))))

(event Collision|EventActorBeginOverlap
  (params (OtherActor :type Actor%20Object%20Reference))
  (|CallParentFunction OtherActor) ; This node is disabled and will not be called.\nDrag off pins to build functionality.
)

(event EventTick
  (params (DeltaSeconds :type Float%20%28single-precision%29)))

(fn ConstructionScript
  (|CallParentFunction)
  (CallFunction|GetTotalNumCars))

(fn Negotiate
  (bind _traffic_light_competitor (Variables|Default|GetTraffic%20Light%20Competitor))
  (return (> (* (Variables|Default|GetPreference%20Factor) (Variables|Default|GetNumber%20of%20Cars%20in%20Street)) (* (Variables|/Game/City/Blueprints/BP_Car_Traffic_Light.BP_Car_Traffic_Light_C|GetPreference%20Factor _traffic_light_competitor) (Variables|BP_Car_Traffic_Light_Leader_C|GetNumber%20of%20Cars%20in%20Street _traffic_light_competitor)))))

(fn GetTotalNumCars
  (bind _output_get (Variables|Default|SetNumber%20of%20Cars%20in%20Street (+ (Variables|/Game/City/Blueprints/BP_Car_Traffic_Light.BP_Car_Traffic_Light_C|GetNumber%20of%20Cars (Variables|Default|GetPartner)) (Variables|Default|GetNumber%20of%20Cars))))
  (Variables|Default|SetUpdated true))

(fn AskCompetitorforUpdate
  (return (Variables|BP_Car_Traffic_Light_Leader_C|GetUpdated (Variables|Default|GetTraffic%20Light%20Competitor))))