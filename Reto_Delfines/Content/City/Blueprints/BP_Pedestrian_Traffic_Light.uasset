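; Pedestrian traffic light actor that shows the opposite signal to a referenced car traffic light.
; Tick polls the car light's CurrentLight, calling TurnGreen when it is red and TurnRed when it is green.
; Both functions swap lit and off materials on the green and red meshes and store the new state, reapplying them every frame rather than only on change.
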(event EventBeginPlay)

(event Collision|EventActorBeginOverlap
  (params (OtherActor :type Actor%20Object%20Reference)))

(event EventTick
  (params (DeltaSeconds :type Float%20%28single-precision%29))
  (switch Utilities|FlowControl|Switch|SwitchonE_Traffic_Lights (Variables|/Game/City/Blueprints/BP_Car_Traffic_Light.BP_Car_Traffic_Light_C|GetCurrent%20light (Variables|Default|GetTraffic%20Light%20Car))
    (:NewEnumerator0
      (CallFunction|TurnGreen))
    (:NewEnumerator2
      (CallFunction|TurnRed))))

(fn ConstructionScript)

(fn TurnGreen
  (Rendering|Material|SetMaterial (Variables|Default|GetGreen1) 0 "/Game/City/Props/Traffic_Lights/PedestrianTrafficLight/M_Green.M_Green")
  (Rendering|Material|SetMaterial (Variables|Default|GetRed1) 0 "/Game/City/Props/Traffic_Lights/M_LightOff.M_LightOff")
  (Variables|Default|SetCurrent%20Light "NewEnumerator2"))

(fn TurnRed
  (Rendering|Material|SetMaterial (Variables|Default|GetGreen1) 0 "/Game/City/Props/Traffic_Lights/M_LightOff.M_LightOff")
  (Rendering|Material|SetMaterial (Variables|Default|GetRed1) 0 "/Game/City/Props/Traffic_Lights/PedestrianTrafficLight/M_Red.M_Red")
  (Variables|Default|SetCurrent%20Light "NewEnumerator0"))