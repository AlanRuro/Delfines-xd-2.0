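; BP_Car_Path is a spline-based traffic lane that spawns BP_Car actors to travel along its path.
; BeginPlay and every Tick attempt a spawn when ActivateSpawn is set and the last car has moved at least OffsetBetweenCars along the spline.
; New cars appear at the first spline point unless colliding, receiving the spline and traffic light.
; The construction script assigns the spline to the first existing car.
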(event Custom|Begin%20Path
  (if (Variables|Default|GetActivate%20Spawn)
    (bind _car_at_begining_ (CallFunction|CheckCaratBegining))
    (if (not _car_at_begining_)
      (CallFunction|SpawnCar))))

(event EventBeginPlay
  (CallFunction|BeginPath))

(event Collision|EventActorBeginOverlap
  (params (OtherActor :type Actor%20Object%20Reference)))

(event EventTick
  (params (DeltaSeconds :type Float%20%28single-precision%29))
  (CallFunction|BeginPath))

(fn ConstructionScript
  (Variables|/Game/City/Blueprints/BP_Car.BP_Car_C|SetPath (Utilities|Array|Get(acopy) (Variables|Default|GetCars)) (Variables|Default|GetSpline)))

(fn CheckCaratBegining
  (bind _cars (Variables|Default|GetCars))
  (return (< (Variables|/Game/City/Blueprints/BP_Car.BP_Car_C|GetDistance%20Along%20Spline (Utilities|Array|Get(acopy) _cars (Utilities|Array|LastIndex _cars))) (Variables|Default|GetOffset%20between%20cars))))

(fn SpawnCar
  (bind _spline (Variables|Default|GetSpline))
  (bind _returnvalue (Spline|GetLocationatSplinePoint _spline 0 "World"))
  (bind _returnvalue_2 (Game|SpawnActorfromClass "/Game/City/Blueprints/BP_Car.BP_Car_C" (Math|Transform|MakeTransform (Math|Vector|MakeVector (.x _returnvalue) (.y _returnvalue) (.z _returnvalue)) (Spline|GetRotationatSplinePoint _spline 0 "World") "1.000000,1.000000,1.000000") "DontSpawnIfColliding" "MultiplyWithRoot" 0 0))
  (Variables|/Game/City/Blueprints/BP_Car.BP_Car_C|SetTraffic%20%20Light%20to%20Follow _returnvalue_2 (Variables|Default|GetTraffic%20Light))
  (Variables|/Game/City/Blueprints/BP_Car.BP_Car_C|SetPath _returnvalue_2 (Variables|Default|GetSpline))
  (Utilities|Array|Add (Variables|Default|GetCars) _returnvalue_2))