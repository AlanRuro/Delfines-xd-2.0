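; BP_Car_Traffic_Light_Follower is a car traffic light that mirrors the state of a Partner light.
; Its construction script runs the parent's, then copies PreferenceFactor and CurrentLight from Partner.
; Every Tick it switches on Partner's CurrentLight and calls the matching TurnRed, TurnYellow or TurnGreen.
; BeginPlay is empty and does not call the parent, nor does Tick.
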(event EventBeginPlay)

(event Collision|EventActorBeginOverlap
  (params (OtherActor :type Actor%20Object%20Reference))
  (|CallParentFunction OtherActor) ; This node is disabled and will not be called.\nDrag off pins to build functionality.
)

(event EventTick
  (params (DeltaSeconds :type Float%20%28single-precision%29))
  (switch Utilities|FlowControl|Switch|SwitchonE_Traffic_Lights (Variables|/Game/City/Blueprints/BP_Car_Traffic_Light.BP_Car_Traffic_Light_C|GetCurrent%20light (Variables|Default|GetPartner))
    (:NewEnumerator0
      (CallFunction|TurnRed))
    (:NewEnumerator1
      (CallFunction|TurnYellow))
    (:NewEnumerator2
      (CallFunction|TurnGreen))))

(fn ConstructionScript
  (bind _partner (Variables|Default|GetPartner))
  (|CallParentFunction)
  (Variables|Default|SetPreference%20Factor (Variables|/Game/City/Blueprints/BP_Car_Traffic_Light.BP_Car_Traffic_Light_C|GetPreference%20Factor _partner))
  (Variables|Default|SetCurrent%20light (Variables|/Game/City/Blueprints/BP_Car_Traffic_Light.BP_Car_Traffic_Light_C|GetCurrent%20light _partner)))