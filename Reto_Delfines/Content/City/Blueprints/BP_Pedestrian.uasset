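; BP_Pedestrian is a city pedestrian that walks along a spline path and obeys an assigned pedestrian traffic light.
; Each tick, Move advances its distance by Speed and snaps it to the spline's location and rotation with a fixed height offset.
; Pawn sensing of its assigned light stops it on red or sets walking speed on green.
; Past the second spline point it speeds up regardless, then destroys itself near the path's end.
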(event OnSeePawn(TrafficLightSensing)
  (params (Pawn :type Pawn%20Object%20Reference))
  (bind _asbp_pedestrian_traffic_light (Utilities|Casting|CastToBP_Pedestrian_Traffic_Light Pawn))
  (if (== _asbp_pedestrian_traffic_light (Variables|Default|GetTraffic%20%20Light%20to%20Follow))
    (switch Utilities|FlowControl|Switch|SwitchonE_Traffic_Lights (Variables|/Game/City/Blueprints/BP_Pedestrian_Traffic_Light.BP_Pedestrian_Traffic_Light_C|GetCurrent%20Light (Variables|Default|GetTraffic%20%20Light%20to%20Follow))
      (:NewEnumerator0
        (Variables|Default|SetSpeed 0.0))
      (:NewEnumerator2
        (Variables|Default|SetSpeed 3e+02)))))

(event EventBeginPlay)

(event Collision|EventActorBeginOverlap
  (params (OtherActor :type Actor%20Object%20Reference)))

(event EventTick
  (params (DeltaSeconds :type Float%20%28single-precision%29))
  (CallFunction|Move DeltaSeconds)
  (if (> (Variables|Default|GetDistance%20Along%20Spline) (Spline|GetDistanceAlongSplineatSplinePoint (Variables|Components|GetPath) 1))
    (Variables|Default|SetSpeed 5e+02)
    (if (< (- (Spline|GetSplineLength (Variables|Components|GetPath)) (Variables|Default|GetDistance%20Along%20Spline)) 5e+01)
      (Actor|DestroyActor))))

(fn ConstructionScript)

(fn Move
  (params (Delta%20Time :type Float%20%28double-precision%29))
  (bind _path (Variables|Components|GetPath))
  (bind _output_get (Variables|Default|SetDistance%20Along%20Spline (+ (Variables|Default|GetDistance%20Along%20Spline) (* (Variables|Default|GetSpeed) Delta%20Time))))
  (Transformation|SetActorLocationAndRotation (Math|Vector|MakeVector (.x (Spline|GetLocationatDistanceAlongSpline _path _output_get "World")) (.y (Spline|GetLocationatDistanceAlongSpline _path _output_get "World")) (+ (.z (Spline|GetLocationatDistanceAlongSpline _path _output_get "World")) -8e+01)) (Spline|GetRotationatDistanceAlongSpline _path _output_get "World")))