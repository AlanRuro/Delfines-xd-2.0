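; Car traffic light actor that cycles endlessly through green, yellow and red on a timer.
; From BeginPlay, a retriggerable delay loop calls LightChange, which switches on CurrentLight to run the next color's function.
; Each Turn function swaps the three lamp materials, records the new state and sets how long it holds before the next change, with yellow the briefest.
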(event Custom|LightChange
  (switch Utilities|FlowControl|Switch|SwitchonE_Traffic_Lights (Variables|Default|GetCurrent%20light)
    (:NewEnumerator0
      (CallFunction|TurnGreen))
    (:NewEnumerator1
      (CallFunction|TurnRed))
    (:NewEnumerator2
      (CallFunction|TurnYellow))))

(event EventBeginPlay
  (CallFunction|LightChange :!label _label)
  (Utilities|FlowControl|RetriggerableDelay (Variables|Default|GetDuration))
  (goto _label))

(event Collision|EventActorBeginOverlap
  (params (OtherActor :type Actor%20Object%20Reference)))

(event EventTick
  (params (DeltaSeconds :type Float%20%28single-precision%29)))

(fn ConstructionScript)

(fn TurnYellow
  (Rendering|Material|SetMaterial (Variables|Default|GetRed) 0 "/Game/City/Props/Traffic_Lights/M_LightOff.M_LightOff")
  (Rendering|Material|SetMaterial (Variables|Default|GetYellow) 0 "/Game/City/Props/Traffic_Lights/PedestrianTrafficLight/M_Yellow.M_Yellow")
  (Rendering|Material|SetMaterial (Variables|Default|GetGreen) 0 "/Game/City/Props/Traffic_Lights/M_LightOff.M_LightOff")
  (Variables|Default|SetCurrent%20light "NewEnumerator1")
  (Variables|Default|SetDuration 1.0))

(fn TurnRed
  (Rendering|Material|SetMaterial (Variables|Default|GetRed) 0 "/Game/City/Props/Traffic_Lights/PedestrianTrafficLight/M_Red.M_Red")
  (Rendering|Material|SetMaterial (Variables|Default|GetYellow) 0 "/Game/City/Props/Traffic_Lights/M_LightOff.M_LightOff")
  (Rendering|Material|SetMaterial (Variables|Default|GetGreen) 0 "/Game/City/Props/Traffic_Lights/M_LightOff.M_LightOff")
  (Variables|Default|SetCurrent%20light "NewEnumerator0")
  (Variables|Default|SetDuration 8.0))

(fn TurnGreen
  (Rendering|Material|SetMaterial (Variables|Default|GetRed) 0 "/Game/City/Props/Traffic_Lights/M_LightOff.M_LightOff")
  (Rendering|Material|SetMaterial (Variables|Default|GetYellow) 0 "/Game/City/Props/Traffic_Lights/M_LightOff.M_LightOff")
  (Rendering|Material|SetMaterial (Variables|Default|GetGreen) 0 "/Game/City/Props/Traffic_Lights/PedestrianTrafficLight/M_Green.M_Green")
  (Variables|Default|SetCurrent%20light "NewEnumerator2")
  (Variables|Default|SetDuration 7.0))