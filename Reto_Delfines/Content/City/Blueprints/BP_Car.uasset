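; City traffic car with a random mesh that drives along a spline Path and destroys itself near the end.
; Before the crossroad it counts itself in its traffic light's car total and takes speed from the light colour seen by pawn sensing.
; Afterwards it leaves the count, stops sensing lights and crosses at fixed speed.
; Sensed cars halt it through a retriggerable-delay flag; pedestrian stopping logic is disconnected.
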(event OnSeePawn(TrafficLightSensing)
  (params (Pawn :type Pawn%20Object%20Reference))
  (if (not (or (Variables|Default|Getis%20Car%20In%20Front?) (Variables|Default|Getis%20Pedestrian%20in%20Front?)))
    (bind _asbp_car_traffic_light (Utilities|Casting|CastToBP_Car_Traffic_Light Pawn))
    (if (== _asbp_car_traffic_light (Variables|Default|GetTraffic%20%20Light%20to%20Follow))
      (switch Utilities|FlowControl|Switch|SwitchonE_Traffic_Lights (Variables|/Game/City/Blueprints/BP_Car_Traffic_Light.BP_Car_Traffic_Light_C|GetCurrent%20light _asbp_car_traffic_light)
        (:NewEnumerator0
          (Variables|Default|SetSpeed 0.0))
        (:NewEnumerator1
          (Variables|Default|SetSpeed 3e+02))
        (:NewEnumerator2
          (Variables|Default|SetSpeed 6e+02))))))

(event OnSeePawn(CarSensing)
  (params (Pawn :type Pawn%20Object%20Reference))
  (Utilities|Casting|CastToBP_Car Pawn)
  (Variables|Default|Setis%20Car%20In%20Front? true)
  (Utilities|FlowControl|Sequence
    (:then_0
      (Variables|Default|SetSpeed 0.0))
    (:then_1
      (Utilities|FlowControl|RetriggerableDelay 0.4)
      (Variables|Default|Setis%20Car%20In%20Front? false))))

(event OnSeePawn(PedestrianSensing)
  (params (Pawn :type Pawn%20Object%20Reference)))

(event EventBeginPlay)

(event Collision|EventActorBeginOverlap
  (params (OtherActor :type Actor%20Object%20Reference)))

(event EventTick
  (params (DeltaSeconds :type Float%20%28single-precision%29))
  (CallFunction|Move DeltaSeconds)
  (bind _is_before_crossroad_ (CallFunction|IsBeforeCrossroad))
  (if _is_before_crossroad_
    (if (not (Variables|Default|GetisConsidered))
      (CallFunction|BeConsidered))
    (else
      (Variables|/Script/AIModule.PawnSensingComponent|SetbSeePawns (Variables|Default|GetTrafficLightSensing) false)
      (bind _is_at_end_ (CallFunction|IsatEnd))
      (if _is_at_end_
        (Variables|Default|SetisConsidered false)
        (CallFunction|AutoDestroy)
        (else
          (if (Variables|Default|GetisConsidered)
            (CallFunction|BeIgnored))
          (CallFunction|CrossStreet))))))

(fn ConstructionScript
  (Components|StaticMesh|SetStaticMesh (Variables|Default|GetStaticMesh) (.OutItem (Utilities|Array|Random (Variables|Default|GetSkin%20Options)))))

(fn Move
  (params (Delta%20Time :type Float%20%28double-precision%29))
  (bind _path (Variables|Default|GetPath))
  (bind _output_get (Variables|Default|SetDistance%20Along%20Spline (+ (Variables|Default|GetDistance%20Along%20Spline) (* (Variables|Default|GetSpeed) Delta%20Time))))
  (Transformation|SetActorLocationAndRotation (Math|Vector|MakeVector (.x (Spline|GetLocationatDistanceAlongSpline _path _output_get "World")) (.y (Spline|GetLocationatDistanceAlongSpline _path _output_get "World")) (+ (.z (Spline|GetLocationatDistanceAlongSpline _path _output_get "World")) -35.0)) (Spline|GetRotationatDistanceAlongSpline _path _output_get "World")))

(fn CrossStreet
  (if (Variables|Default|Getis%20Car%20In%20Front?)
    (Variables|Default|SetSpeed 0.0)
    (else
      (Variables|Default|SetSpeed 8e+02))))

(fn AutoDestroy
  (Actor|DestroyActor))

(fn BeConsidered
  (bind _traffic__light_to_follow (Variables|Default|GetTraffic%20%20Light%20to%20Follow))
  (Variables|/Game/City/Blueprints/BP_Car_Traffic_Light.BP_Car_Traffic_Light_C|SetNumber%20of%20Cars _traffic__light_to_follow (+ (Variables|/Game/City/Blueprints/BP_Car_Traffic_Light.BP_Car_Traffic_Light_C|GetNumber%20of%20Cars _traffic__light_to_follow) 1))
  (Variables|Default|SetisConsidered true))

(fn BeIgnored
  (bind _traffic__light_to_follow (Variables|Default|GetTraffic%20%20Light%20to%20Follow))
  (Variables|/Game/City/Blueprints/BP_Car_Traffic_Light.BP_Car_Traffic_Light_C|SetNumber%20of%20Cars _traffic__light_to_follow (- (Variables|/Game/City/Blueprints/BP_Car_Traffic_Light.BP_Car_Traffic_Light_C|GetNumber%20of%20Cars _traffic__light_to_follow) 1))
  (Variables|Default|SetisConsidered false))

(fn IsBeforeCrossroad
  (return (<= (Variables|Default|GetDistance%20Along%20Spline) (Spline|GetDistanceAlongSplineatSplinePoint (Variables|Default|GetPath) 1))))

(fn IsatEnd
  (return (< (- (Spline|GetSplineLength (Variables|Default|GetPath)) (Variables|Default|GetDistance%20Along%20Spline)) 5e+01)))